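; Title screen game mode that, on BeginPlay, covers the start with a loading screen before presenting the title menu.
; After a short delay it plays the loading widget's fade-out, removing that widget once the animation finishes.
; As the fade starts, it switches the player view to the first CineCameraActor found in the level, adds the title screen widget and shows the mouse cursor.
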(event `self.ReceiveBeginPlay`
  (bind _returnvalue (`|CreateWidget` "/Game/LoadingScreen/WB_LoadingScreen.WB_LoadingScreen_C"))
  (`UserWidget.AddToViewport` _returnvalue 0)
  (`KismetSystemLibrary.Delay` 2.0)
  (`|PlayAnimation` _returnvalue (`/Game/LoadingScreen/WB_LoadingScreen.FadeOut` _returnvalue)
    (:`then`
      (bind _outactors (`GameplayStatics.GetAllActorsOfClass` "/Script/CinematicCamera.CineCameraActor"))
      (`PlayerController.SetViewTargetWithBlend` (`GameplayStatics.GetPlayerController` 0) (`|GetArrayItem` _outactors) 0.0 "VTBlend_Linear" 0.0 false)
      (bind _returnvalue_2 (`|CreateWidget` "/Game/TitleScreen/WBP_TitleScreen.WBP_TitleScreen_C"))
      (`UserWidget.AddToViewport` _returnvalue_2 0)
      (set `PlayerController.bShowMouseCursor` true (`GameplayStatics.GetPlayerController` 0)))
    (:`Finished`
      (`Widget.RemoveFromParent` _returnvalue))))

(fn `UserConstructionScript`)